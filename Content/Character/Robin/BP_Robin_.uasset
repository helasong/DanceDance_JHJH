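; Robin character Blueprint that feeds head orientation into the MPC_Character material parameter collection, for use by materials.
; Each Tick reads the world-space head bone rotation from SKRobinShader and writes its axes as the HeadUp, HeadForward and HeadRight vectors.
; The bone's axes are remapped: forward becomes up, right becomes forward, and up becomes right.
; The construction script makes SKRobinShader1 follow SKRobinShader's pose through a leader pose component.
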(event `self.ReceiveTick`
  (params (DeltaSeconds :type "Float (single-precision)"))
  (bind _rotation (.rotation (`SkinnedMeshComponent.GetBoneTransform` (`self.SK_Robin_Shader`) "head" "RTS_World")))
  (`KismetMaterialLibrary.SetVectorParameterValue` "/Game/Character/Materials/MPC_Character.MPC_Character" "HeadUp" (`KismetMathLibrary.Conv_VectorToLinearColor` (`KismetMathLibrary.GetForwardVector` _rotation)))
  (`KismetMaterialLibrary.SetVectorParameterValue` "/Game/Character/Materials/MPC_Character.MPC_Character" "HeadForward" (`KismetMathLibrary.Conv_VectorToLinearColor` (`KismetMathLibrary.GetRightVector` _rotation)))
  (`KismetMaterialLibrary.SetVectorParameterValue` "/Game/Character/Materials/MPC_Character.MPC_Character" "HeadRight" (`KismetMathLibrary.Conv_VectorToLinearColor` (`KismetMathLibrary.GetUpVector` _rotation))))

(fn `UserConstructionScript`
  (`SkinnedMeshComponent.SetLeaderPoseComponent` (`self.SK_Robin_Shader1`) (`self.SK_Robin_Shader`) false false))