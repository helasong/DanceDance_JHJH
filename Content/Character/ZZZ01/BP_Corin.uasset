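; BP_Corin is a character Blueprint that feeds orientation data to materials and drives an outline mesh.
; Each Tick it writes the world-space axes of the pelvis bone to MPC_Character2 as HeadUp, HeadForward and HeadRight.
; The axes are remapped (forward to up, right to forward, up to right), and the pelvis stands in for the head.
; The construction script makes the Outline mesh follow SkeletalMesh's pose through a leader pose component.
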(event `self.ReceiveTick`
  (params (DeltaSeconds :type "Float (single-precision)"))
  (bind _rotation (.rotation (`SkinnedMeshComponent.GetBoneTransform` (`self.SkeletalMesh`) "pelvis" "RTS_World")))
  (`KismetMaterialLibrary.SetVectorParameterValue` "/Game/Character/Materials/MPC_Character2.MPC_Character2" "HeadUp" (`KismetMathLibrary.Conv_VectorToLinearColor` (`KismetMathLibrary.GetForwardVector` _rotation)))
  (`KismetMaterialLibrary.SetVectorParameterValue` "/Game/Character/Materials/MPC_Character2.MPC_Character2" "HeadForward" (`KismetMathLibrary.Conv_VectorToLinearColor` (`KismetMathLibrary.GetRightVector` _rotation)))
  (`KismetMaterialLibrary.SetVectorParameterValue` "/Game/Character/Materials/MPC_Character2.MPC_Character2" "HeadRight" (`KismetMathLibrary.Conv_VectorToLinearColor` (`KismetMathLibrary.GetUpVector` _rotation))))

(fn `UserConstructionScript`
  (`SkinnedMeshComponent.SetLeaderPoseComponent` (`self.Outline`) (`self.SkeletalMesh`) false false))