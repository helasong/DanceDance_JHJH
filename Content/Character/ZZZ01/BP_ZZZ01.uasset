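; Character Blueprint for ZZZ01 that feeds the head orientation of its SMZZZ01 mesh to materials.
; Every Tick it reads the world-space transform of the head bone (頭) and writes its axes to HeadUp, HeadForward and HeadRight in MPC_Character2.
; The axes are remapped to the bone's orientation: bone forward becomes head up, right becomes head forward, and up becomes head right.
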(event `self.ReceiveTick`
  (params (DeltaSeconds :type "Float (single-precision)"))
  (bind _rotation (.rotation (`SkinnedMeshComponent.GetBoneTransform` (`self.SM_ZZZ01`) "頭" "RTS_World")))
  (`KismetMaterialLibrary.SetVectorParameterValue` "/Game/Character/Materials/MPC_Character2.MPC_Character2" "HeadUp" (`KismetMathLibrary.Conv_VectorToLinearColor` (`KismetMathLibrary.GetForwardVector` _rotation)))
  (`KismetMaterialLibrary.SetVectorParameterValue` "/Game/Character/Materials/MPC_Character2.MPC_Character2" "HeadForward" (`KismetMathLibrary.Conv_VectorToLinearColor` (`KismetMathLibrary.GetRightVector` _rotation)))
  (`KismetMaterialLibrary.SetVectorParameterValue` "/Game/Character/Materials/MPC_Character2.MPC_Character2" "HeadRight" (`KismetMathLibrary.Conv_VectorToLinearColor` (`KismetMathLibrary.GetUpVector` _rotation))))

(fn `UserConstructionScript`)