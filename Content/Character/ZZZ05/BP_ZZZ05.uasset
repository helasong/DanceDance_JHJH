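; Character Blueprint for ZZZ05 that publishes head orientation vectors to the MPC_Character3 material parameter collection for materials to read.
; Every Tick, it reads the world rotation of the SMZZZ05 bone `_dummy_肩C_R_end`, a shoulder-named dummy bone serving as the head reference.
; The bone's forward, up and right axes are remapped to HeadRight, HeadForward and HeadUp respectively.
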(event `self.ReceiveTick`
  (params (DeltaSeconds :type "Float (single-precision)"))
  (bind _rotation (.rotation (`SkinnedMeshComponent.GetBoneTransform` (`self.SM_ZZZ05`) "_dummy_肩C_R_end" "RTS_World")))
  (`KismetMaterialLibrary.SetVectorParameterValue` "/Game/Character/Materials/MPC_Character3.MPC_Character3" "HeadRight" (`KismetMathLibrary.Conv_VectorToLinearColor` (`KismetMathLibrary.GetForwardVector` _rotation)))
  (`KismetMaterialLibrary.SetVectorParameterValue` "/Game/Character/Materials/MPC_Character3.MPC_Character3" "HeadForward" (`KismetMathLibrary.Conv_VectorToLinearColor` (`KismetMathLibrary.GetUpVector` _rotation)))
  (`KismetMaterialLibrary.SetVectorParameterValue` "/Game/Character/Materials/MPC_Character3.MPC_Character3" "HeadUp" (`KismetMathLibrary.Conv_VectorToLinearColor` (`KismetMathLibrary.GetRightVector` _rotation))))

(fn `UserConstructionScript`)